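; Player hero character with camera-relative movement, a visible mouse cursor and left-click attacks that either fire a gun or punch.
; A SpawnGun flag checked on Tick spawns GunBP onto the GunSocket.
; Armed clicks start firing and move a spawned MousePointBP to the cursor hit, while unarmed construction attaches spheres to both hands.
; Death disables input, then after a delay destroys gun and hero and restarts the level.
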(event `self.ReceiveTick`
  (params (DeltaSeconds :type "Float (single-precision)"))
  (if (`self.spawnGun`)
    (bind _returnvalue (`|SpawnActorFromClass` "/Game/weapon/GunBP.GunBP_C" (`SceneComponent.K2_GetComponentToWorld` (`self.Mesh`)) "Undefined" "OverrideRootScale"))
    (bind _output_get (set `self.Gun` _returnvalue))
    (`self.K2_AttachToComponent` _output_get (`self.Mesh`) "GunSocket" "SnapToTarget" "SnapToTarget" "KeepRelative" true)
    (set `self.spawnGun` false)))

(event `self.ReceiveBeginPlay`
  (bind _returnvalue (`|SpawnActorFromClass` "/Game/UI/MousePointBP.MousePointBP_C" (`KismetMathLibrary.Conv_VectorToTransform` (`self.K2_GetActorLocation`)) "Undefined" "OverrideRootScale"))
  (set `self.MouseClickPoint` _returnvalue)
  (set `PlayerController.bShowMouseCursor` true (`GameplayStatics.GetPlayerController` 0)))

(event `InputAction|LeftMouseClicked`
  (params (Key :type "Key Structure" :default "AnyKey"))
  (bind _gun (`self.Gun`))
  (:`Pressed`
    (if (`self.havegun?`)
      (`/Game/weapon/GunBP.StartFiring` _gun)
      (`self.K2_SetActorLocation` (`self.MouseClickPoint`) (`.Location` (`GameplayStatics.BreakHitResult` (`PlayerController.GetHitResultUnderCursorByChannel` (`GameplayStatics.GetPlayerController` 0) "TraceTypeQuery1" true))) false false)
      (else
        (set `self.punching?` true))))
  (:`Released`
    (set `self.punching?` false)
    (`/Game/weapon/GunBP.StopFiring` _gun)))

(event `InputAxis|moveFrontBack`
  (params (AxisValue :type "Float (single-precision)"))
  (`self.AddMovementInput` (`SceneComponent.GetForwardVector` (`self.Camera`)) AxisValue))

(event `InputAxis|moveLeftRight`
  (params (AxisValue :type "Float (single-precision)"))
  (`self.AddMovementInput` (`SceneComponent.GetRightVector` (`self.Camera`)) AxisValue))

(event `Death`
  (set `self.die` true)
  (`self.DisableInput` null)
  (`KismetSystemLibrary.Delay` 1.5)
  (`self.K2_DestroyActor` (`self.Gun`))
  (`self.K2_DestroyActor` self)
  (`KismetSystemLibrary.ExecuteConsoleCommand` "restartlevel"))

(fn `UserConstructionScript`
  (bind _mesh (`self.Mesh`))
  (if (not (`self.havegun?`))
    (`SceneComponent.K2_AttachToComponent` (`self.RightSphere`) _mesh "hand_r" "SnapToTarget" "SnapToTarget" "KeepRelative" true)
    (`SceneComponent.K2_AttachToComponent` (`self.LeftSphere`) _mesh "hand_l" "SnapToTarget" "SnapToTarget" "KeepRelative" true)))